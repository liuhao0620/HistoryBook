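; BP_WarPlayerController is a player controller that shows the mouse cursor, enables click events and moves the controlled pawn with the mouse.
; MouseX input shifts the pawn along world Y and MouseY along world X, inverted and scaled by a fixed factor, with Z unchanged.
; Each move sets the location directly without sweep, and is neither gated by a button nor scaled by delta time.
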(event EventBeginPlay
  (Variables|Default|SetbShowMouseCursor true)
  (Variables|Default|SetbEnableClickEvents true))

(event Collision|EventActorBeginOverlap
  (params (OtherActor :type Actor%20Object%20Reference)))

(event EventTick
  (params (DeltaSeconds :type Float%20%28single-precision%29)))

(event Input|MouseEvents|MouseX
  (params (AxisValue :type Float%20%28single-precision%29))
  (bind _returnvalue (Pawn|GetControlledPawn))
  (bind _returnvalue_2 (Transformation|GetActorLocation _returnvalue))
  (bind (_x _y _z) (Math|Vector|BreakVector _returnvalue_2))
  (if (!= AxisValue 0.0)
    (Utilities|IsValid _returnvalue
      (:Is%20Valid
        (Transformation|SetActorLocation _returnvalue (Math|Vector|MakeVector _x (+ (* AxisValue -1e+02) _y) _z) false false)))))

(event Input|MouseEvents|MouseY
  (params (AxisValue :type Float%20%28single-precision%29))
  (bind _returnvalue (Pawn|GetControlledPawn))
  (bind _returnvalue_2 (Transformation|GetActorLocation _returnvalue))
  (bind (_x _y _z) (Math|Vector|BreakVector _returnvalue_2))
  (if (!= AxisValue 0.0)
    (Utilities|IsValid _returnvalue
      (:Is%20Valid
        (Transformation|SetActorLocation _returnvalue (Math|Vector|MakeVector (+ (* AxisValue -1e+02) _x) _y _z) false false)))))

(fn ConstructionScript)